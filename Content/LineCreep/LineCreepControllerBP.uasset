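; AI controller for a lane creep that sends its pawn toward a point from an indexed Points list.
; Shortly after BeginPlay, TakeTargetPoint bounds-checks the current index and supplies the destination to AIMoveTo.
; A successful move increments the index but does not itself start the next move, and a failed move prints a debug message.
; The LineCreep behavior tree call is disconnected, so it never runs.
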(event `LineGoing`
  (bind (_newparam _success) (`self.TakeTargetPoint` :!label _label))
  (if _success
    (`|AIMoveTo` (`self.K2_GetPawn`) _newparam null
      (:`OnSuccess`
        (`/Engine/EditorBlueprintResources/StandardMacros.IncrementInt` (`self.NumberOfCurrentPoint`)))
      (:`OnFail`
        (`KismetSystemLibrary.PrintString` "FAIL")))))

(event `self.ReceiveBeginPlay`
  (`KismetSystemLibrary.Delay` 0.2)
  (goto _label))

(fn `TakeTargetPoint`
  (returns (NewParam :type "Vector Structure") (Success :type Boolean))
  (bind _points (`self.Points`))
  (bind _numberofcurrentpoint (`self.NumberOfCurrentPoint`))
  (bind (_output_x _output_y _output_z) (`KismetMathLibrary.BreakVector` (`|GetArrayItem` _points _numberofcurrentpoint)))
  (`KismetSystemLibrary.PrintString` "Takepoint")
  (`KismetSystemLibrary.PrintString` (`KismetStringLibrary.Conv_IntToString` _numberofcurrentpoint))
  (if (and (>= _numberofcurrentpoint 0) (< _numberofcurrentpoint (`KismetArrayLibrary.Array_Length` _points)))
    (`KismetSystemLibrary.PrintString` "Hello" true true (struct :`A` 1.0))
    (return (`KismetMathLibrary.MakeVector` _output_x _output_y _output_z) true)
    (else
      (return (0.0 0.0 0.0) false))))

(fn `UserConstructionScript`)