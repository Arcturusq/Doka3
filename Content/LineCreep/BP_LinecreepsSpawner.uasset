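; BP_LinecreepsSpawner is a spawner actor that creates line creeps and gives each a route to follow.
; On BeginPlay it spawns CreepClassRef at its own transform until CountOfCreeps reaches zero, all in one loop with no delay.
; Each creep's controller is cast to LineCreepControllerBP and receives every TargetLocations entry in its Points array, with debug prints along the way.
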(event `self.ReceiveBeginPlay`
  (bind _countofcreeps (`self.CountOfCreeps`))
  (while (> _countofcreeps 0)
    (`/Engine/EditorBlueprintResources/StandardMacros.DecrementInt` _countofcreeps
      (:`  `
        (bind _returnvalue (`|SpawnActorFromClass` (`self.CreepClassRef`) (`self.GetTransform`) "Undefined" "OverrideRootScale" null null))
        (bind _asline_creep_controller_bp (cast `/Game/LineCreep/LineCreepControllerBP` (`Pawn.GetController` _returnvalue)))
        (bind _output_get (set `self.Line Creep Controller BP` _asline_creep_controller_bp))
        (`KismetSystemLibrary.PrintString` "LindeCodasdascS")
        (for _array_element (`self.TargetLocations`)
          (`KismetArrayLibrary.Array_Add` (`/Game/LineCreep/LineCreepControllerBP.Points` _output_get) (`KismetMathLibrary.MakeVector` (.x _array_element) (.y _array_element) (.z _array_element)))
          (`KismetSystemLibrary.PrintString` "qeqewq" true true (struct :`R` 1.0 :`G` 0.739841 :`A` 1.0)))))))

(fn `UserConstructionScript`)